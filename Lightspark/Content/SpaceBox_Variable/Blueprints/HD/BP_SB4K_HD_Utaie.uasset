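; BP_SB4K_HD_Utaie is a space box actor for the HD Utaie variant, built from six face components.
; Its construction script applies the Scale variable to the whole actor.
; It then assigns a matching Utaie material to material slot 0 of each face: Up, Down, Left, Right, Front and Back.
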(fn ConstructionScript
  (Transformation|SetActorScale3D (Variables|Default|GetScale))
  (Rendering|Material|SetMaterial (Variables|Default|GetUp) 0 "/Game/SpaceBox_Variable/Materials/HD/Utaie/Mat_HD_Utaie_Up.Mat_HD_Utaie_Up")
  (Rendering|Material|SetMaterial (Variables|Default|GetRight) 0 "/Game/SpaceBox_Variable/Materials/HD/Utaie/Mat_HD_Utaie_Right.Mat_HD_Utaie_Right")
  (Rendering|Material|SetMaterial (Variables|Default|GetLeft) 0 "/Game/SpaceBox_Variable/Materials/HD/Utaie/Mat_HD_Utaie_Left.Mat_HD_Utaie_Left")
  (Rendering|Material|SetMaterial (Variables|Default|GetFront) 0 "/Game/SpaceBox_Variable/Materials/HD/Utaie/Mat_HD_Utaie_Front.Mat_HD_Utaie_Front")
  (Rendering|Material|SetMaterial (Variables|Default|GetDown) 0 "/Game/SpaceBox_Variable/Materials/HD/Utaie/Mat_HD_Utaie_Down.Mat_HD_Utaie_Down")
  (Rendering|Material|SetMaterial (Variables|Default|GetBack) 0 "/Game/SpaceBox_Variable/Materials/HD/Utaie/Mat_HD_Utaie_Back.Mat_HD_Utaie_Back"))