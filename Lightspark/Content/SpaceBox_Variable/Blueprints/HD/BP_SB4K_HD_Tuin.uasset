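; BP_SB4K_HD_Tuin is a skybox actor that displays the HD "Tuin" space box from six separate face components.
; Its construction script scales the actor by a Scale variable, then assigns a dedicated material to each of the Up, Down, Left, Right, Front and Back faces.
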(fn ConstructionScript
  (Transformation|SetActorScale3D (Variables|Default|GetScale))
  (Rendering|Material|SetMaterial (Variables|Default|GetUp) 0 "/Game/SpaceBox_Variable/Materials/HD/Tuin/Mat_HD_Tuin_Up.Mat_HD_Tuin_Up")
  (Rendering|Material|SetMaterial (Variables|Default|GetRight) 0 "/Game/SpaceBox_Variable/Materials/HD/Tuin/Mat_HD_Tuin_Right.Mat_HD_Tuin_Right")
  (Rendering|Material|SetMaterial (Variables|Default|GetLeft) 0 "/Game/SpaceBox_Variable/Materials/HD/Tuin/Mat_HD_Tuin_Left.Mat_HD_Tuin_Left")
  (Rendering|Material|SetMaterial (Variables|Default|GetFront) 0 "/Game/SpaceBox_Variable/Materials/HD/Tuin/Mat_HD_Tuin_Front.Mat_HD_Tuin_Front")
  (Rendering|Material|SetMaterial (Variables|Default|GetDown) 0 "/Game/SpaceBox_Variable/Materials/HD/Tuin/Mat_HD_Tuin_Down.Mat_HD_Tuin_Down")
  (Rendering|Material|SetMaterial (Variables|Default|GetBack) 0 "/Game/SpaceBox_Variable/Materials/HD/Tuin/Mat_HD_Tuin_Back.Mat_HD_Tuin_Back"))