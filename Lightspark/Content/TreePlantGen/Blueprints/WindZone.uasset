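; WindZone is an actor that takes control of the wind animation of trees inside a sphere of configurable radius.
; After a short BeginPlay delay for the camera controller, it claims overlapping uncontrolled trees and deactivates their branch animation skeletons as an optimization.
; It then sets each tree's animation play rate and invisibility culling, and makes the sphere ignore collision.
; Events forward speed, strength and direction changes to assigned trees.
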(event Custom|ChangeStrength
  (params (newStrength :type Float%20%28single-precision%29))
  (Default|ChangeWindStrength (Variables|Default|GetassignedTrees) newStrength)
  (Variables|Default|SetwindStrength newStrength))

(event Custom|ChangeSpeed
  (params (newSpeed :type Float%20%28single-precision%29))
  (Default|ChangeWindSpeed (Variables|Default|GetassignedTrees) newSpeed)
  (Variables|Default|SetwindSpeed newSpeed))

(event Custom|ChangeDirection
  (params (NewDirection :type Vector))
  (Default|ChangeWindDirection (Variables|Default|GetassignedTrees) NewDirection))

(event EventBeginPlay
  (Utilities|FlowControl|Delay 0.1) ; Important - it must wait for camera controller to make 'IsInCameraViewRange' work ok
  (for _array_element (Collision|GetOverlappingActors (Variables|Default|GetZone) "/Game/TreePlantGen/Blueprints/InternalLogic/Tree.Tree_C" :!class /Script/Engine.PrimitiveComponent)
    (bind _astree (Utilities|Casting|CastToTree _array_element))
    (if (not (Variables|/Game/TreePlantGen/Blueprints/InternalLogic/Tree.Tree_C|GetisUnderWindZoneControl _astree))
      (Utilities|Array|AddUnique (Variables|Default|GetassignedTrees) _astree)
      (Variables|/Game/TreePlantGen/Blueprints/InternalLogic/Tree.Tree_C|SetassignedWindZone _astree self)
      (Variables|/Game/TreePlantGen/Blueprints/InternalLogic/Tree.Tree_C|SetisUnderWindZoneControl _astree true)
      (for _array_element_2 (Variables|/Game/TreePlantGen/Blueprints/InternalLogic/Tree.Tree_C|GetactiveBranches _astree)
        (Components|Activation|Deactivate (Variables|/Game/TreePlantGen/Blueprints/InternalLogic/Branch.Branch_C|GetAnimationSkeleton _array_element_2)) ; Optimization. If will activate it again when needed, for example in Start/Stop Animation functions or Impulse function.
      )))
  (for _array_element_3 (Variables|Default|GetassignedTrees)
    (Utilities|FlowControl|Sequence
      (:then_0
        (Components|Timeline|SetPlayRate (Variables|/Game/TreePlantGen/Blueprints/InternalLogic/Tree.Tree_C|GetWindAnimTimeline_Var1 _array_element_3) (Variables|Default|GetwindSpeed))
        (Variables|/Game/TreePlantGen/Blueprints/InternalLogic/Tree.Tree_C|SetcullAnimIfInvisible _array_element_3 (Variables|Default|GetCullAnimationOnInvisibleTrees)))
      (:then_1
        (Default|CheckingifCullAnimationON/OFF _array_element_3 true))))
  (Collision|SetCollisionResponsetoAllChannels (Variables|Default|GetZone) "ECR_Ignore"))

(fn ConstructionScript
  (Components|Sphere|SetSphereRadius (Variables|Default|GetZone) (Variables|Default|GetRadius) false))