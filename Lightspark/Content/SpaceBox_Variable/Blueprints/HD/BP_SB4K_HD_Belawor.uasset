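; Space box Blueprint for the HD Belawor variant, forming a backdrop from six face components: Up, Down, Left, Right, Front and Back.
; The construction script sets the actor's 3D scale from the Scale variable.
; It then assigns each face its matching Belawor material in slot 0, with no further logic in the graph.
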(fn ConstructionScript
  (Transformation|SetActorScale3D (Variables|Default|GetScale))
  (Rendering|Material|SetMaterial (Variables|Default|GetUp) 0 "/Game/SpaceBox_Variable/Materials/HD/Belawor/Mat_HD_Belawor_Up.Mat_HD_Belawor_Up")
  (Rendering|Material|SetMaterial (Variables|Default|GetRight) 0 "/Game/SpaceBox_Variable/Materials/HD/Belawor/Mat_HD_Belawor_Right.Mat_HD_Belawor_Right")
  (Rendering|Material|SetMaterial (Variables|Default|GetLeft) 0 "/Game/SpaceBox_Variable/Materials/HD/Belawor/Mat_HD_Belawor_Left.Mat_HD_Belawor_Left")
  (Rendering|Material|SetMaterial (Variables|Default|GetFront) 0 "/Game/SpaceBox_Variable/Materials/HD/Belawor/Mat_HD_Belawor_Front.Mat_HD_Belawor_Front")
  (Rendering|Material|SetMaterial (Variables|Default|GetDown) 0 "/Game/SpaceBox_Variable/Materials/HD/Belawor/Mat_HD_Belawor_Down.Mat_HD_Belawor_Down")
  (Rendering|Material|SetMaterial (Variables|Default|GetBack) 0 "/Game/SpaceBox_Variable/Materials/HD/Belawor/Mat_HD_Belawor_Back.Mat_HD_Belawor_Back"))