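; BP_SB4K_HD_Omxos is a space skybox actor showing the HD Omxos variant through six face components.
; Its construction script sets the actor's scale from the Scale variable.
; It then assigns a dedicated Omxos material to the first slot of each Up, Down, Left, Right, Front and Back component.
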(fn ConstructionScript
  (Transformation|SetActorScale3D (Variables|Default|GetScale))
  (Rendering|Material|SetMaterial (Variables|Default|GetUp) 0 "/Game/SpaceBox_Variable/Materials/HD/Omxos/Mat_HD_Omxos_Up.Mat_HD_Omxos_Up")
  (Rendering|Material|SetMaterial (Variables|Default|GetRight) 0 "/Game/SpaceBox_Variable/Materials/HD/Omxos/Mat_HD_Omxos_Right.Mat_HD_Omxos_Right")
  (Rendering|Material|SetMaterial (Variables|Default|GetLeft) 0 "/Game/SpaceBox_Variable/Materials/HD/Omxos/Mat_HD_Omxos_Left.Mat_HD_Omxos_Left")
  (Rendering|Material|SetMaterial (Variables|Default|GetFront) 0 "/Game/SpaceBox_Variable/Materials/HD/Omxos/Mat_HD_Omxos_Front.Mat_HD_Omxos_Front")
  (Rendering|Material|SetMaterial (Variables|Default|GetDown) 0 "/Game/SpaceBox_Variable/Materials/HD/Omxos/Mat_HD_Omxos_Down.Mat_HD_Omxos_Down")
  (Rendering|Material|SetMaterial (Variables|Default|GetBack) 0 "/Game/SpaceBox_Variable/Materials/HD/Omxos/Mat_HD_Omxos_Back.Mat_HD_Omxos_Back"))