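; BP_SB4K_HD_Phipa is a space skybox actor for the HD Phipa variant in the SpaceBox_Variable content.
; Its construction script sets the actor's 3D scale from the Scale variable.
; It then assigns a dedicated Phipa material to slot 0 of each of the six face components: Up, Down, Left, Right, Front and Back.
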(fn ConstructionScript
  (Transformation|SetActorScale3D (Variables|Default|GetScale))
  (Rendering|Material|SetMaterial (Variables|Default|GetUp) 0 "/Game/SpaceBox_Variable/Materials/HD/Phipa/Mat_HD_Phipa_Up.Mat_HD_Phipa_Up")
  (Rendering|Material|SetMaterial (Variables|Default|GetRight) 0 "/Game/SpaceBox_Variable/Materials/HD/Phipa/Mat_HD_Phipa_Right.Mat_HD_Phipa_Right")
  (Rendering|Material|SetMaterial (Variables|Default|GetLeft) 0 "/Game/SpaceBox_Variable/Materials/HD/Phipa/Mat_HD_Phipa_Left.Mat_HD_Phipa_Left")
  (Rendering|Material|SetMaterial (Variables|Default|GetFront) 0 "/Game/SpaceBox_Variable/Materials/HD/Phipa/Mat_HD_Phipa_Front.Mat_HD_Phipa_Front")
  (Rendering|Material|SetMaterial (Variables|Default|GetDown) 0 "/Game/SpaceBox_Variable/Materials/HD/Phipa/Mat_HD_Phipa_Down.Mat_HD_Phipa_Down")
  (Rendering|Material|SetMaterial (Variables|Default|GetBack) 0 "/Game/SpaceBox_Variable/Materials/HD/Phipa/Mat_HD_Phipa_Back.Mat_HD_Phipa_Back"))