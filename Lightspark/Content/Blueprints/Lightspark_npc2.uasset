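; Lightspark NPC that wanders to random reachable points within a radius and moves toward player-tagged components entering its EnemySight trigger.
; AIMoveTo results loop through a delay back into the trigger-and-tag check, choosing chase or wander; a successful chase ends the loop.
; Leaving sight stops movement and computes a path to the spawn position, but the following AIMoveTo has no pawn or destination wired.
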(event OnComponentBeginOverlap(EnemySight)
  (params (OtherActor :type Actor%20Object%20Reference) (OtherComp :type Primitive%20Component%20Object%20Reference) (OtherBodyIndex :type Integer) (bFromSweep :type Boolean) (SweepResult :type Hit%20Result%20Structure%20%28by%20ref%29))
  (bind _self self)
  ;[1 1 1] Follow
  (Variables|Default|SetInTrigger true)
  (if (and (Components|ComponentHasTag OtherComp "Player") (Variables|Default|GetInTrigger)) :!label _label
    (AI|AIMoveTo _self "0, 0, 0" OtherActor 5.0 false
      (:OnFail
        _))
    (else
      ;[1 1 1] Movement
      (AI|AIMoveTo _self (AI|Navigation|GetRandomReachablePointinRadius (Transformation|GetActorLocation) 1e+03) 0 5.0 false
        (:OnSuccess
          _)
        (:OnFail
          _))))
  (Utilities|FlowControl|Delay 2.0)
  (goto _label))

(event OnComponentEndOverlap(EnemySight)
  (params (OtherActor :type Actor%20Object%20Reference) (OtherComp :type Primitive%20Component%20Object%20Reference) (OtherBodyIndex :type Integer))
  (bind _returnvalue (Transformation|GetActorLocation))
  (bind _self self)
  ;[1 1 1] Follow
  (Variables|Default|SetInTrigger false)
  (Components|Movement|StopMovementImmediately (Variables|Character|GetCharacterMovement))
  (bind _returnvalue_2 (Class|NavigationSystem|FindPathtoLocationSynchronously _returnvalue (Variables|Default|GetStartPosition)))
  (AI|AIMoveTo _returnvalue_2 0 "0, 0, 0" 0 5.0 false
    (:OnSuccess
      (Utilities|FlowControl|Delay 2.0 :!label _label)
      (if (and (Components|ComponentHasTag (stale OnComponentBeginOverlap(EnemySight) OtherComp) "Player") (Variables|Default|GetInTrigger))
        (AI|AIMoveTo _self "0, 0, 0" (stale OnComponentBeginOverlap(EnemySight) OtherActor) 5.0 false
          (:OnFail
            (goto _label)))
        (else
          ;[1 1 1] Movement
          (AI|AIMoveTo _self (AI|Navigation|GetRandomReachablePointinRadius _returnvalue 1e+03) 0 5.0 false
            (:OnSuccess
              (goto _label))
            (:OnFail
              (goto _label))))))))

(event EventBeginPlay
  (bind _returnvalue (Transformation|GetActorLocation))
  (bind _self self)
  ;[1 1 1] Movement
  (Variables|Default|SetStartPosition _returnvalue)
  (Utilities|FlowControl|Delay 1.0)
  (AI|AIMoveTo _self (AI|Navigation|GetRandomReachablePointinRadius _returnvalue 1e+03) 0 5.0 false :!label _label
    (:OnSuccess
      _)
    (:OnFail
      _))
  (Utilities|FlowControl|Delay 2.0 :!label _label_2)
  ;[1 1 1] Follow
  (if (and (Components|ComponentHasTag (stale OnComponentBeginOverlap(EnemySight) OtherComp) "Player") (Variables|Default|GetInTrigger))
    (AI|AIMoveTo _self "0, 0, 0" (stale OnComponentBeginOverlap(EnemySight) OtherActor) 5.0 false
      (:OnFail
        (goto _label_2)))
    (else
      (goto _label))))

(fn ConstructionScript)