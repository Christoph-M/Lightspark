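; Face is a puzzle-gated actor whose mesh rotates when the player approaches, once all linked pillars are triggered.
; Trigger polls every entry in Pillars, sets Activate only if all report triggered, then boosts emissive on both meshes.
; While active, a player capsule overlapping the Box enables Tick, which rolls StaticMesh at constant speed until world roll reaches -90 degrees, then disables Tick.
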(event OnComponentBeginOverlap(Box)
  (params (OtherActor :type Actor%20Object%20Reference) (OtherComp :type Primitive%20Component%20Object%20Reference) (OtherBodyIndex :type Integer) (bFromSweep :type Boolean) (SweepResult :type Hit%20Result%20Structure%20%28by%20ref%29))
  (if (Variables|Default|GetActivate)
    (Utilities|Casting|CastToPlayerCharacter OtherActor)
    (Utilities|Casting|CastToCapsuleComponent OtherComp)
    (Actor|Tick|SetActorTickEnabled true)))

(event EventTick
  (params (DeltaSeconds :type Float%20%28single-precision%29))
  (Transformation|AddLocalRotation (Variables|Default|GetStaticMesh) (* (Math|Rotator|MakeRotator -3e+01 0.0 0.0) DeltaSeconds) false false)
  (if (<= (.Roll (Math|Rotator|BreakRotator (Transformation|GetWorldRotation (Variables|Default|GetStaticMesh)))) -9e+01)
    (Actor|Tick|SetActorTickEnabled false)))

(fn ConstructionScript)

(fn Trigger
  (Variables|Default|SetToBeActivated true)
  (for _array_element (Variables|Default|GetPillars)
    (bind _returnvalue (Class|TriggeredActor|HasBeenTriggered _array_element))
    (if (not _returnvalue)
      (Variables|Default|SetToBeActivated false)))
  (bind _output_get (Variables|Default|SetActivate (Variables|Default|GetToBeActivated)))
  (if _output_get
    (Rendering|Material|SetScalarParameterValueonMaterials (Variables|Default|GetStaticMesh1) "EmissiveBoost" 1e+01)))