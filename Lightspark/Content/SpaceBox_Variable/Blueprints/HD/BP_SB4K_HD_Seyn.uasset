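; BP_SB4K_HD_Seyn is a space skybox actor for the Seyn variant in the HD SpaceBox set.
; Its construction script sets the actor's scale from the Scale variable.
; It then assigns a dedicated Seyn material to the first material slot of each of the six face components: Up, Down, Left, Right, Front and Back.
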(fn ConstructionScript
  (Transformation|SetActorScale3D (Variables|Default|GetScale))
  (Rendering|Material|SetMaterial (Variables|Default|GetUp) 0 "/Game/SpaceBox_Variable/Materials/HD/Seyn/Mat_HD_Seyn_Up.Mat_HD_Seyn_Up")
  (Rendering|Material|SetMaterial (Variables|Default|GetRight) 0 "/Game/SpaceBox_Variable/Materials/HD/Seyn/Mat_HD_Seyn_Right.Mat_HD_Seyn_Right")
  (Rendering|Material|SetMaterial (Variables|Default|GetLeft) 0 "/Game/SpaceBox_Variable/Materials/HD/Seyn/Mat_HD_Seyn_Left.Mat_HD_Seyn_Left")
  (Rendering|Material|SetMaterial (Variables|Default|GetFront) 0 "/Game/SpaceBox_Variable/Materials/HD/Seyn/Mat_HD_Seyn_Front.Mat_HD_Seyn_Front")
  (Rendering|Material|SetMaterial (Variables|Default|GetDown) 0 "/Game/SpaceBox_Variable/Materials/HD/Seyn/Mat_HD_Seyn_Down.Mat_HD_Seyn_Down")
  (Rendering|Material|SetMaterial (Variables|Default|GetBack) 0 "/Game/SpaceBox_Variable/Materials/HD/Seyn/Mat_HD_Seyn_Back.Mat_HD_Seyn_Back"))