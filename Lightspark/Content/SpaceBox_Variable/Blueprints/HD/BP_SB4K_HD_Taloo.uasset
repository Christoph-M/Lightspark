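; BP_SB4K_HD_Taloo is a space box Blueprint that displays the HD Taloo backdrop on six directional face components.
; Its construction script scales the actor by the Scale variable, then assigns each face (Up, Down, Left, Right, Front, Back) its matching Taloo material in slot 0.
; The file holds no other logic, so all setup happens at construction.
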(fn ConstructionScript
  (Transformation|SetActorScale3D (Variables|Default|GetScale))
  (Rendering|Material|SetMaterial (Variables|Default|GetUp) 0 "/Game/SpaceBox_Variable/Materials/HD/Taloo/Mat_HD_Taloo_Up.Mat_HD_Taloo_Up")
  (Rendering|Material|SetMaterial (Variables|Default|GetRight) 0 "/Game/SpaceBox_Variable/Materials/HD/Taloo/Mat_HD_Taloo_Right.Mat_HD_Taloo_Right")
  (Rendering|Material|SetMaterial (Variables|Default|GetLeft) 0 "/Game/SpaceBox_Variable/Materials/HD/Taloo/Mat_HD_Taloo_Left.Mat_HD_Taloo_Left")
  (Rendering|Material|SetMaterial (Variables|Default|GetFront) 0 "/Game/SpaceBox_Variable/Materials/HD/Taloo/Mat_HD_Taloo_Front.Mat_HD_Taloo_Front")
  (Rendering|Material|SetMaterial (Variables|Default|GetDown) 0 "/Game/SpaceBox_Variable/Materials/HD/Taloo/Mat_HD_Taloo_Down.Mat_HD_Taloo_Down")
  (Rendering|Material|SetMaterial (Variables|Default|GetBack) 0 "/Game/SpaceBox_Variable/Materials/HD/Taloo/Mat_HD_Taloo_Back.Mat_HD_Taloo_Back"))