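; CloseEnough is a Behavior Tree decorator condition for AI run by Follow_AI_CONT, gating on distance to a follow target.
; It casts the owner to that controller, then measures the distance between its controlled pawn and the TargetToFollow blackboard actor.
; Despite its name, it passes when that distance is at least AcceptableDistance, meaning the pawn is not yet close enough.
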(fn PerformConditionCheck
  (params (OwnerActor :type Actor%20Object%20Reference))
  (bind _asfollow_ai_cont (Utilities|Casting|CastToFollow_AI_CONT OwnerActor))
  (Variables|Default|SetAI%20Controller%20Reference _asfollow_ai_cont)
  (return (>= (Math|Vector|VectorLength (- (Transformation|GetActorLocation (AI|BehaviorTree|GetBlackboardValueasActor (Variables|Default|GetTargetToFollow))) (Transformation|GetActorLocation (Pawn|GetControlledPawn (Variables|Default|GetAI%20Controller%20Reference))))) (Variables|Default|GetAcceptableDistance))))