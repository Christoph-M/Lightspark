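; BP_SB4K_HD_Ephrims is a space skybox actor for the HD Ephrims variant, built from six face components.
; Its construction script scales the whole actor by the Scale variable.
; It then assigns a dedicated Ephrims material to the first material slot of each Up, Down, Left, Right, Front and Back face.
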(fn ConstructionScript
  (Transformation|SetActorScale3D (Variables|Default|GetScale))
  (Rendering|Material|SetMaterial (Variables|Default|GetUp) 0 "/Game/SpaceBox_Variable/Materials/HD/Ephrims/Mat_HD_Ephrims_Up.Mat_HD_Ephrims_Up")
  (Rendering|Material|SetMaterial (Variables|Default|GetRight) 0 "/Game/SpaceBox_Variable/Materials/HD/Ephrims/Mat_HD_Ephrims_Right.Mat_HD_Ephrims_Right")
  (Rendering|Material|SetMaterial (Variables|Default|GetLeft) 0 "/Game/SpaceBox_Variable/Materials/HD/Ephrims/Mat_HD_Ephrims_Left.Mat_HD_Ephrims_Left")
  (Rendering|Material|SetMaterial (Variables|Default|GetFront) 0 "/Game/SpaceBox_Variable/Materials/HD/Ephrims/Mat_HD_Ephrims_Front.Mat_HD_Ephrims_Front")
  (Rendering|Material|SetMaterial (Variables|Default|GetDown) 0 "/Game/SpaceBox_Variable/Materials/HD/Ephrims/Mat_HD_Ephrims_Down.Mat_HD_Ephrims_Down")
  (Rendering|Material|SetMaterial (Variables|Default|GetBack) 0 "/Game/SpaceBox_Variable/Materials/HD/Ephrims/Mat_HD_Ephrims_Back.Mat_HD_Ephrims_Back"))