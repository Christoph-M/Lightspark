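; AggroCheck is an AI behavior tree tick node that finds visible targets for a Follow_AI_CONT-controlled pawn.
; Each tick it sphere-traces around the pawn, ignoring all AI_Char actors, then line-traces to each hit to confirm line of sight.
; Visible hits set TargetToFollow and TargetLocation, while blocked hits clear only TargetToFollow, so the last hit processed wins.
; Both traces leave persistent debug drawing.
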(event EventTick
  (params (OwnerActor :type Actor%20Object%20Reference) (DeltaSeconds :type Float%20%28single-precision%29))
  ;[1 1 1] Is AI Controller Set?
  (if (!= (Variables|Default|GetAI%20Controller%20Reference) 0)
    _
    (else
      (bind _asfollow_ai_cont (Utilities|Casting|CastToFollow_AI_CONT OwnerActor))
      (Variables|Default|SetAI%20Controller%20Reference _asfollow_ai_cont)))
  (bind _outactors (Actor|GetAllActorsOfClass "/Game/Blueprints/AI/AI_Char.AI_Char_C"))
  (Variables|Default|SetMyLocation (Transformation|GetActorLocation (Pawn|GetControlledPawn (Variables|Default|GetAI%20Controller%20Reference))))
  (bind _outhits (Collision|MultiSphereTraceForObjects (Transformation|GetActorLocation (Pawn|GetControlledPawn (Variables|Default|GetAI%20Controller%20Reference))) (+ (Transformation|GetActorLocation (Pawn|GetControlledPawn (Variables|Default|GetAI%20Controller%20Reference))) "0, 0,15.000000") 5e+02 (Variables|Default|GetDesiredObjectTypes) false _outactors "Persistent"))
  (bind _array_element (Utilities|Array|ForEachLoopwithBreak _outhits)
    (:LoopBody
      (bind _outhit (Collision|LineTraceByChannel (Variables|Default|GetMyLocation) (Transformation|GetActorLocation (.HitActor (Collision|BreakHitResult _array_element))) "TraceTypeQuery1" false _outactors "Persistent"))
      (if (== (.HitActor (Collision|BreakHitResult _outhit)) (.HitActor (Collision|BreakHitResult _array_element)))
        (Class|BTFunctionLibrary|SetBlackboardValueasObject (Variables|Default|GetTargetToFollow) (.HitActor (Collision|BreakHitResult _outhit)))
        (AI|BehaviorTree|SetBlackboardValueasVector (Variables|Default|GetTargetLocation) (Transformation|GetActorLocation (.HitActor (Collision|BreakHitResult _outhit))))
        (else
          (Class|BTFunctionLibrary|SetBlackboardValueasObject (Variables|Default|GetTargetToFollow)))))))