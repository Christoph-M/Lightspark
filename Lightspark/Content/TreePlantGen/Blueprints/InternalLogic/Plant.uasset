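; Procedural plant actor that sways away from or with impulses and hides itself beyond a cull distance.
; Construction script builds a randomized tapered spline-mesh stem, then scatters instanced leaf meshes along it, tinting those with names ending in COLOR.
; Overlaps or ReactToImpulse calls temporarily reparent the spline to AnimationParent, which a timeline rotates by strength and elasticity.
; A randomized looping timer toggles visibility by distance to the player camera manager.
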(event OnComponentBeginOverlap(Collider)
  (params (OtherActor :type Actor%20Object%20Reference) (OtherComp :type Primitive%20Component%20Object%20Reference) (OtherBodyIndex :type Integer) (bFromSweep :type Boolean) (SweepResult :type Hit%20Result%20Structure%20%28by%20ref%29))
  (if (> (Utilities|Time|GetGameTimeinSeconds) 1.0)
    (CallFunction|ReacttoImpulse (* (Math|Rotator|GetRotationXVector (Math|Rotator|FindLookatRotation (Transformation|GetActorLocation OtherActor) (Transformation|GetActorLocation))) -1) (* (Variables|Default|GetreactToObjectsStrength) (Variables|Default|Getelasticity)))))

(event Custom|CheckIfCull
  (if (< (Transformation|GetDistanceTo (Game|GetPlayerCameraManager 0)) (Variables|Default|GetCullDistance))
    (if (Variables|Default|GetisHidden)
      (Rendering|SetActorHiddenInGame false)
      (Variables|Default|SetisHidden false))
    (elif (not (Variables|Default|GetisHidden))
      (Rendering|SetActorHiddenInGame true)
      (Variables|Default|SetisHidden true))))

(event Custom|CheckingIfCull_ON/OFF
  (params (ON/OFF :type Boolean))
  (if ON/OFF
    (bind _returnvalue (Utilities|Time|SetTimerbyEvent (delegate Custom|CheckIfCull) (Math|Random|RandomFloatinRange 2.0 3.0) true))
    (Variables|Default|Settimer_CheckIfCull _returnvalue)
    (else
      (Class|KismetSystemLibrary|ClearTimerHandle (Variables|Default|Gettimer_CheckIfCull)))))

(event Custom|ReactToImpulse
  (params (impulseDirection :type Vector) (impulseStrength :type Float%20%28single-precision%29))
  (bind _returnvalue (Transformation|GetActorLocation))
  (bind _returnvalue_2 (Transformation|GetActorTransform))
  (bind _returnvalue_3 (Math|Transform|InverseTransformLocation _returnvalue_2 _returnvalue))
  (bind _returnvalue_4 (+ _returnvalue impulseDirection))
  (bind _returnvalue_5 (Math|Transform|InverseTransformLocation _returnvalue_2 _returnvalue_4))
  (bind _returnvalue_6 (Math|Rotator|FindLookatRotation _returnvalue_3 _returnvalue_5))
  (bind _returnvalue_7 (Math|Rotator|MakeRotator (.roll _returnvalue_6) (.pitch _returnvalue_6) (.yaw _returnvalue_6)))
  (if (not (Variables|Default|GetanimIsPlaying))
    (Variables|Default|SetimpulseStrength impulseStrength)
    (Variables|Default|SetanimIsPlaying true)
    (Transformation|SetRelativeRotation (Variables|Default|GetanimationParent) _returnvalue_7 false false)
    (Variables|Default|SetrotationBeforeImpulse _returnvalue_7)
    (Class|SceneComponent|Attachto (Variables|Default|GetSpline) (Variables|Default|GetanimationParent) "None" "KeepWorldPosition" true)
    (Variables|Default|SetimpulseRotation (Math|Rotator|MakeRotator (.roll _returnvalue_6) (+ (.pitch _returnvalue_6) (* (Variables|Default|GetimpulseStrength) (Variables|Default|GetElasticity))) (.yaw _returnvalue_6)))
    (bind _alpha (Timeline|ImpulseAnim_Var1 PlayFromStart)
      (:Update
        (Transformation|SetRelativeRotation (Variables|Default|GetanimationParent) (Math|Rotator|Lerp(Rotator) (Variables|Default|GetrotationBeforeImpulse) (Variables|Default|GetimpulseRotation) _alpha) false false))
      (:Finished
        (Variables|Default|SetanimIsPlaying false)
        (Class|SceneComponent|Attachto (Variables|Default|GetSpline) (Variables|Default|GetDefaultSceneRoot) "None" "KeepWorldPosition" true)))))

(event EventBeginPlay
  (Utilities|FlowControl|Delay 0.5)
  (CallFunction|CheckifCull)
  (CallFunction|CheckingifCullON/OFF true))

(fn ConstructionScript
  (bind _spline (Variables|Default|GetSpline))
  (bind _spline_2 (Variables|Default|GetSpline))
  (bind _spline_3 (Variables|Default|GetSpline))
  (bind _curviness (Variables|Default|Getcurviness))
  (bind _spline_4 (Variables|Default|GetSpline))
  (bind _startscale (Variables|Default|GetstartScale))
  (bind _endscale (Variables|Default|GetendScale))
  (bind _plantheight (Variables|Default|GetplantHeight))
  (bind _returnvalue (* _curviness -1.0))
  (bind _returnvalue_2 (* _startscale 0.7))
  (bind _returnvalue_3 (Math|Random|RandomFloatinRange _returnvalue _curviness))
  (bind _returnvalue_4 (Math|Vector2D|MakeVector2D _returnvalue_2 _returnvalue_2))
  (Utilities|FlowControl|Sequence
    (:then_0
      (Spline|ClearSplinePoints _spline_2)
      (Spline|AddSplinePoint _spline_2 (Math|Vector|MakeVector 0.0 0.0 -2.0) "Local")
      (for _index (range 0 (Variables|Default|GetcurveAmount))
        (LocalVariables|SetheightOfThePreviousPoint (+ (LocalVariables|GetheightOfThePreviousPoint) (Math|Random|RandomFloatinRange (- _plantheight 2e+01) _plantheight)))
        (Spline|AddSplinePoint _spline_2 (Math|Vector|MakeVector _returnvalue_3 _returnvalue_3 (LocalVariables|GetheightOfThePreviousPoint)) "Local")
        (bind _returnvalue_5 (AddComponent|AddSplineMeshComponent true))
        (Rendering|Material|SetMaterial _returnvalue_5 0 (Variables|Default|GetstemMaterial))
        (Class|SceneComponent|Attachto _returnvalue_5 (Variables|Default|GetSpline) "None" "KeepRelativeOffset" false)
        (SplineMesh|SetStartandEnd _returnvalue_5 (.Location (Spline|GetLocationandTangentatSplinePoint _spline_3 _index "Local")) (.Tangent (Spline|GetLocationandTangentatSplinePoint _spline_3 _index "Local")) (.Location (Spline|GetLocationandTangentatSplinePoint _spline_3 (+ _index 1) "Local")) (.Tangent (Spline|GetLocationandTangentatSplinePoint _spline_3 (+ _index 1) "Local")) true :!class /Script/Engine.SplineMeshComponent)
        (if (== _index 0)
          (SplineMesh|SetStartScale _returnvalue_5 (Math|Vector2D|MakeVector2D _startscale _startscale) true :!class /Script/Engine.SplineMeshComponent)
          (SplineMesh|SetEndScale _returnvalue_5 (Math|Vector2D|MakeVector2D _returnvalue_2 _returnvalue_2) true :!class /Script/Engine.SplineMeshComponent)
          (elif (== _index (Variables|Default|GetcurveAmount))
            (SplineMesh|SetEndScale _returnvalue_5 (Math|Vector2D|MakeVector2D _endscale _endscale) true :!class /Script/Engine.SplineMeshComponent)
            (SplineMesh|SetStartScale _returnvalue_5 (Math|Vector2D|MakeVector2D _returnvalue_2 _returnvalue_2) true :!class /Script/Engine.SplineMeshComponent)
            (else
              (SplineMesh|SetStartScale _returnvalue_5 _returnvalue_4 true :!class /Script/Engine.SplineMeshComponent)
              (SplineMesh|SetEndScale _returnvalue_5 _returnvalue_4 true :!class /Script/Engine.SplineMeshComponent))))))
    (:then_1
      (for _array_element (Variables|Default|GetLeaves)
        (bind _returnvalue_6 (AddComponent|AddInstancedStaticMeshComponent false))
        (Components|StaticMesh|SetStaticMesh _returnvalue_6 (.Type (Utilities|Struct|BreakPlantLeafs _array_element)))
        (Class|SceneComponent|Attachto _returnvalue_6 (Variables|Default|GetSpline) "None" "KeepRelativeOffset" false)
        (for _index_2 (range 1 (.Amount (Utilities|Struct|BreakPlantLeafs _array_element)))
          (Components|InstancedStaticMesh|AddInstance _returnvalue_6 (Math|Transform|MakeTransform (select (.fixedGrowHeight (Utilities|Struct|BreakPlantLeafs _array_element)) (Spline|GetLocationatDistanceAlongSpline _spline_4 (Math|Float|MapRangeClamped (Math|Random|RandomFloatinRange (- (.growHeight (Utilities|Struct|BreakPlantLeafs _array_element)) (.growHeightTolerance (Utilities|Struct|BreakPlantLeafs _array_element))) (+ (.growHeight (Utilities|Struct|BreakPlantLeafs _array_element)) (.growHeightTolerance (Utilities|Struct|BreakPlantLeafs _array_element)))) 0.0 1.0 0.0 (Spline|GetSplineLength _spline_4)) "Local") (Spline|GetLocationatDistanceAlongSpline _spline (Math|Random|RandomFloatinRange 1e+01 (Spline|GetSplineLength _spline)) "Local")) (Math|Rotator|MakeRotator (Math|Random|RandomFloatinRange (- (.Angle (Utilities|Struct|BreakPlantLeafs _array_element)) 5.0) (+ (.Angle (Utilities|Struct|BreakPlantLeafs _array_element)) 5.0)) (Math|Random|RandomFloatinRange -1e+01 1e+01) (Math|Random|RandomFloatinRange 0.0 3.6e+02)) (Math|Vector|MakeVector (Math|Random|RandomFloatinRange (* (.Scale (Utilities|Struct|BreakPlantLeafs _array_element)) 0.7) (.Scale (Utilities|Struct|BreakPlantLeafs _array_element))) (Math|Random|RandomFloatinRange (* (.Scale (Utilities|Struct|BreakPlantLeafs _array_element)) 0.7) (.Scale (Utilities|Struct|BreakPlantLeafs _array_element))) (Math|Random|RandomFloatinRange (* (.Scale (Utilities|Struct|BreakPlantLeafs _array_element)) 0.7) (.Scale (Utilities|Struct|BreakPlantLeafs _array_element))))))
          (if (Utilities|Enum|Equal(Enum) (Utilities|Array|Get(acopy) (Utilities|String|ParseIntoArray (Utilities|GetDisplayName (.Type (Utilities|Struct|BreakPlantLeafs _array_element))) "_") (- (Utilities|Array|Length (Utilities|String|ParseIntoArray (Utilities|GetDisplayName (.Type (Utilities|Struct|BreakPlantLeafs _array_element))) "_")) 1)) "COLOR")
            (bind _returnvalue_7 (Rendering|Material|CreateDynamicMaterialInstance _returnvalue_6 0 (Rendering|Material|GetMaterial _returnvalue_6 0) :!class /Script/Engine.PrimitiveComponent))
            (Rendering|Material|SetVectorParameterValue _returnvalue_7 "Color" (.Color (Utilities|Struct|BreakPlantLeafs _array_element)) :!class /Script/Engine.MaterialInstanceDynamic)
            (Rendering|Material|SetScalarParameterValue _returnvalue_7 "Glow" (.ColorGlow (Utilities|Struct|BreakPlantLeafs _array_element)) :!class /Script/Engine.MaterialInstanceDynamic)
            (Rendering|Material|SetMaterial _returnvalue_6 0 _returnvalue_7)))))))