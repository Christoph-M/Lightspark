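; Enemy AI character that plays particle effects when it is disabled.
; The Disabled event spawns a VoidTotPopp burst and an Absaugen (suction) emitter at the capsule, the latter with pitch forced to 90 degrees.
; Unconnected leftover nodes would spawn another EnemyAiCharacter with a behavior tree and copy waypoints through its AI_Controller, but they never run.
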(event EventDestroyed)

(event EventTick
  (params (DeltaSeconds :type Float%20%28single-precision%29)))

(event EventActorBeginOverlap
  (params (OtherActor :type Actor%20Object%20Reference)))

(event EventBeginPlay)

(event EventDisabled
  (bind _capsulecomponent (Variables|Default|GetCapsuleComponent))
  (bind _returnvalue (Transformation|GetWorldLocation _capsulecomponent))
  (bind _returnvalue_2 (Transformation|GetWorldRotation _capsulecomponent))
  (bind (_roll _pitch _yaw) (Math|Rotator|BreakRotator _returnvalue_2))
  (Effects|SpawnEmitteratLocation "/Game/Particles/Effects/VoidTotPopp.VoidTotPopp" _returnvalue _returnvalue_2)
  (Effects|SpawnEmitteratLocation "/Game/Particles/Effects/Absaugen.Absaugen" _returnvalue (Math|Rotator|MakeRotator _roll 9e+01 _yaw)))

(fn ConstructionScript)