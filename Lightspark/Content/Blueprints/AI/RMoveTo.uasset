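; Behavior tree task that moves the AI-controlled pawn to the actor stored in the TargetToFollow blackboard key.
; On execute it caches the owner as a Follow_AI_CONT controller if not already set, then runs AIMoveTo on its pawn.
; A successful move finishes the task as failed (false), while a failed move has no handler and never calls FinishExecute.
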(event EventReceiveExecute
  (params (OwnerActor :type Actor%20Object%20Reference))
  (if (!= (Variables|Default|GetAI%20Controller%20Reference) 0)
    _
    (else
      (bind _asfollow_ai_cont (Utilities|Casting|CastToFollow_AI_CONT OwnerActor))
      (Variables|Default|SetAI%20Controller%20Reference _asfollow_ai_cont)))
  (AI|AIMoveTo (Pawn|GetControlledPawn (Variables|Default|GetAI%20Controller%20Reference)) "0, 0, 0" (AI|BehaviorTree|GetBlackboardValueasActor (Variables|Default|GetTargetToFollow)) 5.0 false
    (:OnSuccess
      (AI|BehaviorTree|FinishExecute false))))