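; Triggered blockade actor that moves down along its local Z axis once triggered.
; Tick is off from BeginPlay until Trigger enables it, then each frame applies a fixed, non-swept offset unscaled by delta time.
; A countdown set at BeginPlay delays the parent Trigger call.
; On expiry tick is re-enabled rather than disabled, so the movement and parent call repeat every frame.
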(event EventBeginPlay
  (Actor|Tick|SetActorTickEnabled false)
  (Variables|Default|SetTimer 4.0))

(event EventActorBeginOverlap
  (params (OtherActor :type Actor%20Object%20Reference)))

(event EventTick
  (params (DeltaSeconds :type Float%20%28single-precision%29))
  (Transformation|AddActorLocalOffset "0, 0,-40.000000" false false)
  (bind _output_get (Variables|Default|SetTimer (- (Variables|Default|GetTimer) DeltaSeconds)))
  (if (<= _output_get 0.0)
    (Actor|Tick|SetActorTickEnabled true)
    (|CallParentFunction (stale EventTrigger OtherActor))))

(event EventTrigger
  (params (OtherActor :type Actor%20Object%20Reference))
  (Actor|Tick|SetActorTickEnabled true))

(fn ConstructionScript)