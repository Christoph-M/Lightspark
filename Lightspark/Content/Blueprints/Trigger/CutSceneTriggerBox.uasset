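; A trigger box that plays a Matinee cutscene when the player character's capsule overlaps it.
; While active, it freezes the player by setting custom time dilation to zero and starts the referenced CutScene.
; After a delay equal to the Matinee's length, it restores normal time dilation and deactivates itself.
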(event OnComponentBeginOverlap(CollisionComponent)
  (params (OtherActor :type Actor%20Object%20Reference) (OtherComp :type Primitive%20Component%20Object%20Reference) (OtherBodyIndex :type Integer) (bFromSweep :type Boolean) (SweepResult :type Hit%20Result%20Structure%20%28by%20ref%29))
  (bind _cutscene (Variables|Default|GetCutScene))
  (if (Variables|Default|GetActive)
    (bind _asplayer_character (Utilities|Casting|CastToPlayerCharacter OtherActor))
    (Utilities|Casting|CastToCapsuleComponent OtherComp)
    (Variables|/Script/Engine.Actor|SetCustomTimeDilation _asplayer_character 0.0)
    (Audio|Components|Audio|Play _cutscene)
    (Utilities|FlowControl|Delay (Variables|/Script/Engine.InterpData|GetInterpLength (Variables|/Script/Engine.MatineeActor|GetMatineeData _cutscene)))
    (Variables|/Script/Engine.Actor|SetCustomTimeDilation _asplayer_character 1.0)
    (Variables|Default|SetActive false)))

(fn ConstructionScript)