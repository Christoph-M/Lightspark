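; A one-shot trigger box pickup that gives the player character Light Flash charges.
; On begin play it spawns a persistent particle effect at its location, picked from an array by the clamped charge amount.
; When the player's capsule overlaps the box while active, it passes the charge amount to SetLightFlashUses, deactivates and destroys the particle.
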(event OnComponentBeginOverlap(Box)
  (params (OtherActor :type Actor%20Object%20Reference) (OtherComp :type Primitive%20Component%20Object%20Reference) (OtherBodyIndex :type Integer) (bFromSweep :type Boolean) (SweepResult :type Hit%20Result%20Structure%20%28by%20ref%29))
  (if (Variables|Default|GetActive)
    (bind _asplayer_character (Utilities|Casting|CastToPlayerCharacter OtherActor))
    (Utilities|Casting|CastToCapsuleComponent OtherComp)
    (Class|PlayerCharacter|SetLightFlashUses _asplayer_character (Variables|Default|GetChargeIncrease))
    (Variables|Default|SetActive false)
    (Components|DestroyComponent (Variables|Default|GetCurParticle))))

(event EventBeginPlay
  (bind _returnvalue (Effects|SpawnEmitteratLocation (Utilities|Array|Get(acopy) (Variables|Default|GetParticles) (Math|Integer|Clamp(Integer) (- (Variables|Default|GetChargeIncrease) 1) 0 2)) (Transformation|GetActorLocation) "0, 0, 0" false))
  (Variables|Default|SetCurParticle _returnvalue))

(fn ConstructionScript)