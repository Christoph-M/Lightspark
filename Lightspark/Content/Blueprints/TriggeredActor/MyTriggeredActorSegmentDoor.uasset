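; Segmented puzzle door, a triggered actor that shows progress on four plates and lowers itself when activated.
; On Trigger, each lit plate reveals its particle effect and plays a one-time flame sound; with all four lit, a delayed timeline boosts emissive on the door mesh and head.
; ActivateDoor enables Tick to slide the mesh down on a countdown, then calls the parent activation.
; The door-opening sound plays at BeginPlay, not on activation.
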(event EventActivateDoor
  ;[1 1 1] Open Door
  (Actor|Tick|SetActorTickEnabled true))

(event EventTrigger
  (params (OtherActor :type Actor%20Object%20Reference))
  (|CallParentFunction OtherActor)
  (Utilities|FlowControl|Sequence
    (:then_0
      (Utilities|FlowControl|Sequence
        (:then_0
          (if (and (Utilities|Array|Get(acopy) (Variables|Default|GetPlatesLitUp)) (Variables|Default|GetLightUpPlate1))
            (Rendering|SetVisibility (Variables|Default|GetParticleSystem) true false)))
        (:then_1
          (if (and (Utilities|Array|Get(acopy) (Variables|Default|GetPlatesLitUp) 1) (Variables|Default|GetLightUpPlate2))
            (Rendering|SetVisibility (Variables|Default|GetParticleSystem1) true false)))
        (:then_2
          (if (and (Utilities|Array|Get(acopy) (Variables|Default|GetPlatesLitUp) 2) (Variables|Default|GetLightUpPlate3))
            (Rendering|SetVisibility (Variables|Default|GetParticleSystem2) true false)))
        (:then_3
          (if (and (Utilities|Array|Get(acopy) (Variables|Default|GetPlatesLitUp) 3) (Variables|Default|GetLightUpPlate4))
            (Rendering|SetVisibility (Variables|Default|GetParticleSystem3) true false)))))
    (:then_1
      (Utilities|FlowControl|Sequence
        (:then_0
          (if (and (Utilities|Array|Get(acopy) (Variables|Default|GetPlatesLitUp)) (Variables|Default|GetLightUpPlate1))
            (Variables|Default|SetLightUpPlate1 false)
            (Audio|PlaySoundatLocation "/Game/Audio/Environment/Flame_Loop.Flame_Loop" (Transformation|GetActorLocation) "0, 0, 0" 0.5 1.0 0.0 (Variables|Default|GetNewVar_0) :!label _label)))
        (:then_1
          (if (and (Utilities|Array|Get(acopy) (Variables|Default|GetPlatesLitUp) 1) (Variables|Default|GetLightUpPlate2))
            (Variables|Default|SetLightUpPlate2 false)
            (goto _label)))
        (:then_2
          (if (and (Utilities|Array|Get(acopy) (Variables|Default|GetPlatesLitUp) 2) (Variables|Default|GetLightUpPlate3))
            (Variables|Default|SetLightUpPlate3 false)
            (goto _label)))
        (:then_3
          (if (and (Utilities|Array|Get(acopy) (Variables|Default|GetPlatesLitUp) 3) (Variables|Default|GetLightUpPlate4))
            (Variables|Default|SetLightUpPlate4 false)
            (goto _label)))))
    (:then_2
      (if (Math|Boolean|ANDBoolean (Utilities|Array|Get(acopy) (Variables|Default|GetPlatesLitUp)) (Utilities|Array|Get(acopy) (Variables|Default|GetPlatesLitUp) 1) (Utilities|Array|Get(acopy) (Variables|Default|GetPlatesLitUp) 2) (Utilities|Array|Get(acopy) (Variables|Default|GetPlatesLitUp) 3))
        (Utilities|FlowControl|Delay 1.0)
        (bind _emissiveboost (Timeline|LIghtUp PlayFromStart)
          (:Update
            (Rendering|Material|SetScalarParameterValueonMaterials (Variables|Default|GetStaticMesh) "EmissiveBoost" _emissiveboost)))))))

(event EventBeginPlay
  ;[1 1 1] Open Door
  (Actor|Tick|SetActorTickEnabled false)
  (Variables|Default|SetTimer 4.7)
  (Audio|PlaySound2D "/Game/Audio/Environment/Open_Door.Open_Door"))

(event EventTick
  (params (DeltaSeconds :type Float%20%28single-precision%29))
  ;[1 1 1] Open Door
  (Transformation|AddLocalOffset (Variables|Default|GetStaticMesh) (* (Math|Vector|MakeVector 0.0 0.0 -1e+01) DeltaSeconds) false false)
  (bind _output_get (Variables|Default|SetTimer (- (Variables|Default|GetTimer) DeltaSeconds)))
  (if (<= _output_get 0.0)
    (Actor|Tick|SetActorTickEnabled false)
    (|CallParentFunction)))

(fn ConstructionScript)