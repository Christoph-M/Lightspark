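; Impulse source actor that sends a radial shockwave to nearby trees and plants, optionally firing shortly after it spawns.
; Impulse gathers actors overlapping a Range-sized sphere and calls ReactToImpulse on each Tree or Plant, with strength fading by distance.
; Trees also receive a particle rotation and a distance-based reaction delay scaled by shockwave speed.
; A fire impact emitter plays at the source, and construction toggles its light and arrow visibility.
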(event EventBeginPlay
  (Utilities|FlowControl|Delay 0.1)
  (if (Variables|Default|GetfireUponSpawning)
    (CallFunction|Impulse)))

(fn ConstructionScript
  (bind _showlight (Variables|Default|GetshowLight))
  (bind _pointlight (Variables|Default|GetPointLight))
  (Components|Sphere|SetSphereRadius (Variables|Default|GetImpulseRadius) (Variables|Default|GetRange) true)
  (Development|SetHiddeninGame _pointlight (not _showlight) false)
  (Rendering|SetVisibility _pointlight _showlight false)
  (Development|SetHiddeninGame (Variables|Default|GetArrow) (not (Variables|Default|GetshowArrow)) false))

(fn Impulse
  (bind _returnvalue (Transformation|GetActorLocation))
  (bind _impulseradius (Variables|Default|GetImpulseRadius))
  (bind _sphereradius (Variables|/Script/Engine.SphereComponent|GetSphereRadius _impulseradius))
  (for _array_element (Collision|GetOverlappingActors (Variables|Default|GetImpulseRadius) 0 :!class /Script/Engine.PrimitiveComponent)
    (bind _astree (Utilities|Casting|CastToTree _array_element)
      (:then
        (Default|ReacttoImpulse _astree (Math|Rotator|GetRotationXVector (Math|Rotator|FindLookatRotation (Transformation|GetActorLocation _astree) _returnvalue)) (* (Variables|Default|GetStrength) (Math|Float|MapRangeClamped (Transformation|GetDistanceTo _astree) 0.0 _sphereradius 1.0 0.05)) (Math|Rotator|FindLookatRotation _returnvalue (Transformation|GetActorLocation _astree)) (Variables|Default|GetShockwaveSpeedInfluence) (/ (Math|Float|MapRangeClamped (Transformation|GetDistanceTo _astree) 0.0 _sphereradius 0.0 1.0) (Variables|Default|GetShockwaveSpeed))))
      (:CastFailed
        (bind _asplant (Utilities|Casting|CastToPlant _array_element))
        (Default|ReacttoImpulse _asplant (* (Math|Rotator|GetRotationXVector (Math|Rotator|FindLookatRotation (Transformation|GetActorLocation) (Transformation|GetActorLocation _asplant))) -1) (* (Variables|Default|GetStrength) (Math|Float|MapRangeClamped (Transformation|GetDistanceTo _asplant) 0.0 (Variables|/Script/Engine.SphereComponent|GetSphereRadius (Variables|Default|GetImpulseRadius)) 1.0 0.05))))))
  (bind _returnvalue_2 (Effects|SpawnEmitteratLocation "/Game/TreePlantGen/DemoEffects/FX_Mobile/combat/P_Impact_Golem_Death_Fire.P_Impact_Golem_Death_Fire" (Transformation|GetActorLocation)))
  (Transformation|SetWorldScale3D _returnvalue_2 "1.000000,1.000000,1.000000"))